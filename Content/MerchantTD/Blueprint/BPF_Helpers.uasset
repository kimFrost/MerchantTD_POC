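; BPF_Helpers is a Blueprint function library of small array helpers for resources and tiles in MerchantTD.
; It extracts the resource from each container, sums resource prices from their raw data, and averages tile world locations to find a midpoint.
; Each function loops over its input array and skips invalid elements.
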(fn ContainerstoResources
  (params (Containers :type Array%20of%20BP%20Container%20Object%20References))
  (for _array_element Containers
    (Utilities|IsValid _array_element
      (:Is%20Valid
        (Utilities|Array|Add (LocalVariables|Get_Resources) (Variables|/Game/MerchantTD/Blueprint/Actors/BP_Container.BP_Container_C|GetResource _array_element)))))
  (return (LocalVariables|Get_Resources)))

(fn GetResourcesTotalPrice
  (params (Resources :type Array%20of%20U%20Resource%20Object%20References))
  (for _array_element Resources
    (Utilities|IsValid _array_element
      (:Is%20Valid
        (LocalVariables|Set_TotalPrice (+ (LocalVariables|Get_TotalPrice) (.Price (Utilities|Struct|BreakST_Resource (Variables|/Game/MerchantTD/Blueprint/UObjects/UResource.UResource_C|GetRawData _array_element))))))))
  (return (LocalVariables|Get_TotalPrice)))

(fn GetTilesMidPoint
  (params (Tiles :type Array%20of%20U%20Tile%20Object%20References))
  (for _array_element Tiles
    (Utilities|IsValid _array_element
      (:Is%20Valid
        (Utilities|Array|Add (LocalVariables|Get_Locations) (Variables|/Game/MerchantTD/Blueprint/UObjects/UTile.UTile_C|GetWorldLocation _array_element)))))
  (return (Math|Vector|GetVectorArrayAverage (LocalVariables|Get_Locations))))