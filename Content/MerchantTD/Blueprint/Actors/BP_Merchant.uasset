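; BP_Merchant is a merchant actor that walks to a market in the MerchantTD game.
; On BeginPlay it finds all BP_Market actors and has its AI controller issue MoveToLocation toward the first one's location, then breaks out of the loop.
; The movement result is not used, and several alternative movement approaches are left disconnected in the graph.
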(event EventBeginPlay
  (bind _outactors (Actor|GetAllActorsOfClass "/Game/MerchantTD/Blueprint/Actors/BP_Market.BP_Market_C"))
  (bind _array_element (Utilities|Array|ForEachLoopwithBreak _outactors :!label _label)
    (:LoopBody
      (bind _returnvalue (AI|Navigation|MovetoLocation (AI|GetAIController self) (Transformation|GetActorLocation _array_element) -1.0 true true false))
      (goto _label Break))))

(event Collision|EventActorBeginOverlap
  (params (OtherActor :type Actor%20Object%20Reference)))

(event EventTick
  (params (DeltaSeconds :type Float%20%28single-precision%29)))

(fn ConstructionScript)