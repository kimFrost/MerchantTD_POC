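; BP_Market is a market actor that turns arriving merchants into transactions and registers itself with the city.
; It gets the city through the GM_MerchantTD city-created callback.
; When a merchant overlaps its Box, it builds a fixed-total UTransaction, spawns a BP_TransactionVisualizer at the merchant, broadcasts the transaction, then destroys the merchant.
; Tick draws the box as a debug outline every frame.
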(event OnComponentBeginOverlap(Box)
  (params (OverlappedComponent :type Primitive%20Component%20Object%20Reference) (OtherActor :type Actor%20Object%20Reference) (OtherComp :type Primitive%20Component%20Object%20Reference) (OtherBodyIndex :type Integer) (bFromSweep :type Boolean) (SweepResult :type Hit%20Result%20Structure%20%28by%20ref%29))
  (bind _asbp_merchant (Utilities|Casting|CastToBP_Merchant OtherActor))
  (CallFunction|TriggerTransaction _asbp_merchant)
  (Actor|DestroyActor _asbp_merchant))

(event Custom|CustomEvent_0
  (params (City :type U%20City%20Object%20Reference))
  (bind _output_get (Variables|Default|SetCity City))
  (Default|RegisterMarket _output_get self))

(event EventBeginPlay
  (bind _asgm_merchant_td (Utilities|Casting|CastToGM_MerchantTD (Game|GetGameMode)))
  (EventDispatchers|BindEventtoCityCreated _asgm_merchant_td (delegate Custom|CustomEvent_0)))

(event EventTick
  (params (DeltaSeconds :type Float%20%28single-precision%29))
  (bind _box (Variables|Default|GetBox))
  (Rendering|Debug|DrawDebugBox (Transformation|GetWorldLocation _box) (Variables|/Script/Engine.BoxComponent|GetBoxExtent _box) "(R=0.218729,G=0.000000,B=1.000000,A=1.000000)" "0, 0, 0" 0.0 2.0))

(fn ConstructionScript)

(fn TriggerTransaction
  (params (Merchant :type BP%20Merchant%20Object%20Reference))
  (bind _self self)
  (Utilities|IsValid Merchant
    (:Is%20Valid
      (bind _returnvalue (Game|ConstructObjectfromClass "/Game/MerchantTD/Blueprint/UObjects/UTransaction.UTransaction_C" _self Merchant _self 0 1e+01))
      (Game|SpawnActorfromClass "/Game/MerchantTD/Blueprint/Actors/BP_TransactionVisualizer.BP_TransactionVisualizer_C" (Math|Conversions|ToTransform(Vector) (Transformation|GetActorLocation Merchant)) "Undefined" 0 _returnvalue 0)
      (Default|CallOnTransaction _returnvalue))))