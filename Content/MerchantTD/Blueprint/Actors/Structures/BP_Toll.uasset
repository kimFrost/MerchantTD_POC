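; BP_Toll is a toll structure that halts one merchant at a time when it enters its overlap sphere.
; Merchants who have already paid are released to the nearest market, while others start a search timer.
; PayToll charges the stored merchant, triggers a GM_MerchantTD transaction and releases it.
; A container search that destroys merchants carrying illegal resources exists, but its call is disconnected.
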(event OnComponentBeginOverlap(Sphere)
  (params (OverlappedComponent :type Primitive%20Component%20Object%20Reference) (OtherActor :type Actor%20Object%20Reference) (OtherComp :type Primitive%20Component%20Object%20Reference) (OtherBodyIndex :type Integer) (bFromSweep :type Boolean) (SweepResult :type Hit%20Result%20Structure%20%28by%20ref%29))
  (bind _asbp_merchant (Utilities|Casting|CastToBP_Merchant OtherActor))
  (Utilities|IsValid (Variables|Default|GetStoredMerchant)
    (:Is%20Not%20Valid
      (bind _output_get (Variables|Default|SetStoredMerchant _asbp_merchant))
      (AI|Navigation|StopMovement (AI|GetAIController _output_get))
      (CallFunction|SearchMerchant (Variables|Default|GetStoredMerchant)))))

(event Custom|PayTollDelegate_Event
  (params (Merchant :type BP%20Merchant%20Object%20Reference)))

(event Custom|PayToll
  (bind _storedmerchant (Variables|Default|GetStoredMerchant))
  (Utilities|IsValid _storedmerchant
    (:Is%20Valid
      (Default|PayToll _storedmerchant)
      (bind _asgm_merchant_td (Utilities|Casting|CastToGM_MerchantTD (Game|GetGameMode))
        (:then
          (Default|TriggerTransaction _asgm_merchant_td (Variables|Default|GetStoredMerchant)))
        (:CastFailed
          _))
      (CallFunction|ReleaseMerchant))))

(event EventBeginPlay)

(fn ConstructionScript
  (|CallParentFunction))

(fn SearchContainers
  (params (Containers :type Array%20of%20BP%20Container%20Object%20References))
  (for _array_element (CallFunction|ContainerstoResources Containers)
    (Utilities|IsValid _array_element
      (:Is%20Valid
        (if (.Illigal (Utilities|Struct|BreakST_Resource (Variables|/Game/MerchantTD/Blueprint/UObjects/UResource.UResource_C|GetRawData _array_element)))
          (Utilities|IsValid (Variables|Default|GetStoredMerchant)
            (:Is%20Valid
              (Actor|DestroyActor (Variables|Default|GetStoredMerchant))
              (Variables|Default|SetStoredMerchant 0)))
          (else
            (Development|PrintString (.ID (Utilities|Struct|BreakST_Resource (Variables|/Game/MerchantTD/Blueprint/UObjects/UResource.UResource_C|GetRawData _array_element))))))))))

(fn SearchMerchant
  (params (Merchant :type BP%20Merchant%20Object%20Reference))
  (Utilities|IsValid Merchant
    (:Is%20Valid
      (if (Variables|/Game/MerchantTD/Blueprint/Characters/BP_Merchant.BP_Merchant_C|GetHasPayedToll Merchant)
        (CallFunction|ReleaseMerchant)
        (else
          (Utilities|Time|SetTimerbyEvent (EventDispatchers|CreateEvent :!event Custom|PayToll) 4.0))))))

(fn ReleaseMerchant
  (Utilities|IsValid (Variables|Default|GetStoredMerchant)
    (:Is%20Valid
      (Default|GotoNearestMarket (Variables|Default|GetStoredMerchant)))
    (:Is%20Not%20Valid
      _))
  (Variables|Default|SetStoredMerchant 0))