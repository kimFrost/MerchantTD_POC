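; BP_BuilderClass is a builder actor in MerchantTD that previews a set of tiles for structure placement.
; SetTilesOn stores the tiles, and Tick draws a debug plane over each valid one, green or red by its AttachedStructure, plus a purple plane at the actor's own location.
; An unconnected branch would rebuild static mesh components at the tile positions but never runs, so the preview relies entirely on debug drawing.
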(event EventBeginPlay
  (|CallParentFunction))

(event Collision|EventActorBeginOverlap
  (params (OtherActor :type Actor%20Object%20Reference)))

(event EventTick
  (params (DeltaSeconds :type Float%20%28single-precision%29))
  (for _array_element (Variables|Default|GetTiles)
    (Utilities|IsValid _array_element
      (:Is%20Valid
        (Class|KismetSystemLibrary|DrawDebugPlane (Utilities|Struct|MakePlane 1.0 0.0 0.0 1.0) (Variables|/Game/MerchantTD/Blueprint/UObjects/UTile.UTile_C|GetWorldLocation _array_element) (/ (Variables|/Game/MerchantTD/Blueprint/UObjects/UTile.UTile_C|GetSize _array_element) 2.0) (Math|Color|SelectColor "(R=0.060310,G=1.000000,B=0.000000,A=1.000000)" "(R=1.000000,G=0.000000,B=0.015278,A=1.000000)" (== (Variables|/Game/MerchantTD/Blueprint/UObjects/UTile.UTile_C|GetAttachedStructure _array_element) 0)) 0.0))))
  (Class|KismetSystemLibrary|DrawDebugPlane (Utilities|Struct|MakePlane 5.0 0.0 0.0 1.0) (Transformation|GetActorLocation) 5e+01 "(R=0.589264,G=0.000000,B=1.000000,A=1.000000)" 0.0))

(fn ConstructionScript
  (|CallParentFunction))

(fn SetTileson
  (params (Tiles :type Array%20of%20U%20Tile%20Object%20References))
  (bind _output_get (Variables|Default|SetTiles Tiles)))