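; BP_Structure is a structure actor for MerchantTD that occupies tiles on the game mode's grid.
; Its construction script reads its DATA_Structures row by RowName, caches it as RawData, and sizes the NavBlock box and StaticMesh scale from the column and row counts.
; On BeginPlay it registers itself at its location through GM_MerchantTD's AttachStructureToTiles and stores the returned tiles in OnTiles.
; A disconnected debug loop can draw boxes on those tiles.
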(event EventBeginPlay
  (bind _asgm_merchant_td (Utilities|Casting|CastToGM_MerchantTD (Game|GetGameMode)))
  (bind _tiles (Default|AttachStructuretoTiles _asgm_merchant_td self (Transformation|GetActorLocation)))
  (bind _output_get (Variables|Default|SetOnTiles _tiles)))

(fn ConstructionScript
  (bind _returnvalue (Utilities|GetDataTableRow "/Game/MerchantTD/Data/DATA_Structures.DATA_Structures" (Variables|Default|GetRowName))
    (:then
      (bind _output_get (Variables|Default|SetRawData _returnvalue))
      (Components|Box|SetBoxExtent (Variables|Default|GetNavBlock) (Math|Vector|MakeVector (/ (* (.Colums (Utilities|Struct|BreakST_Structure _output_get)) 1e+02) 2.0) (/ (* (.Rows (Utilities|Struct|BreakST_Structure _output_get)) 1e+02) 2.0) 1e+02) true)
      (Transformation|SetWorldScale3D (Variables|Default|GetStaticMesh) (Math|Vector|MakeVector (* (.Colums (Utilities|Struct|BreakST_Structure _output_get)) 1e+02) (* (.Rows (Utilities|Struct|BreakST_Structure _output_get)) 1e+02) 0.0)))))