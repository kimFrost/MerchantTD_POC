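; Merchant character for MerchantTD that carries a randomly chosen resource to a market and can pay a toll to the city.
; On BeginPlay it fills its child-actor container with a random DATA_Resources row, then sends its AI controller to the first BP_Market found, not necessarily the nearest.
; PayToll adds the cargo's total price to the GameMode's City funds and sets HasPayedToll, which colours a debug plane drawn every tick.
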(event EventBeginPlay
  (Utilities|FlowControl|Sequence
    (:then_0
      (CallFunction|AsignRandResource))
    (:then_1
      (bind _outactors (Actor|GetAllActorsOfClass "/Game/MerchantTD/Blueprint/Actors/BP_Market.BP_Market_C"))
      (bind _array_element (Utilities|Array|ForEachLoopwithBreak _outactors :!label _label)
        (:LoopBody
          (bind _returnvalue (AI|Navigation|MovetoLocation (AI|GetAIController self) (Transformation|GetActorLocation _array_element) -1.0 true true false))
          (goto _label Break))))))

(event EventTick
  (params (DeltaSeconds :type Float%20%28single-precision%29))
  (CallFunction|DrawDebugs))

(fn ConstructionScript)

(fn AsignRandResource
  (bind _asbp_container (Utilities|Casting|CastToBP_Container (Variables|/Script/Engine.ChildActorComponent|GetChildActor (Variables|Default|GetBP_Container))))
  (bind _outrownames (DataTable|GetDataTableRowNames "/Game/MerchantTD/Data/DATA_Resources.DATA_Resources"))
  (bind _returnvalue (Utilities|GetDataTableRow "/Game/MerchantTD/Data/DATA_Resources.DATA_Resources" (Utilities|Array|Get(acopy) _outrownames (Math|Random|RandomIntegerinRange 0 (- (Utilities|Array|Length _outrownames) 1))))
    (:then
      (bind _returnvalue_2 (Game|ConstructObjectfromClass "/Game/MerchantTD/Blueprint/UObjects/UResource.UResource_C" _asbp_container _returnvalue))
      (Variables|/Game/MerchantTD/Blueprint/Actors/BP_Container.BP_Container_C|SetResource _asbp_container _returnvalue_2)
      (Utilities|Array|Add (Variables|Default|GetContainers) _asbp_container))))

(fn GotoNearestMarket
  (bind _outactors (Actor|GetAllActorsOfClass "/Game/MerchantTD/Blueprint/Actors/BP_Market.BP_Market_C"))
  (bind _array_element (Utilities|Array|ForEachLoopwithBreak _outactors :!label _label)
    (:LoopBody
      (bind _returnvalue (AI|Navigation|MovetoLocation (AI|GetAIController self) (Transformation|GetActorLocation _array_element) -1.0 true true false))
      (goto _label Break))))

(fn PayToll
  (bind _asgm_merchant_td (Utilities|Casting|CastToGM_MerchantTD (Game|GetGameMode)))
  (Utilities|IsValid (Variables|/Game/MerchantTD/Blueprint/Gamemodes/GM_MerchantTD.GM_MerchantTD_C|GetCity _asgm_merchant_td)
    (:Is%20Valid
      (Default|AddFunds (Variables|/Game/MerchantTD/Blueprint/Gamemodes/GM_MerchantTD.GM_MerchantTD_C|GetCity _asgm_merchant_td) (CallFunction|GetResourcesTotalPrice (CallFunction|ContainerstoResources (Variables|Default|GetContainers))))
      (Variables|Default|SetHasPayedToll true))))

(fn DrawDebugs
  (Class|KismetSystemLibrary|DrawDebugPlane (Utilities|Struct|MakePlane 2e+02 0.0 0.0 1.0) (Transformation|GetActorLocation) 5e+01 (Math|Color|SelectColor "(R=0.190461,G=1.000000,B=0.000000,A=1.000000)" "(R=1.000000,G=0.024480,B=0.000000,A=1.000000)" (Variables|Default|GetHasPayedToll)) 0.0))