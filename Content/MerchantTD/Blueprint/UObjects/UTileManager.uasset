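; Tile manager that builds and holds the grid of UTile objects for MerchantTD.
; CreateTiles loops over rows and columns, constructing each tile with its grid coordinates and a world location offset by half the grid size around the origin, then adds it to Tiles.
; WorldLocationToTile is unfinished: it only prints the input location, leaving its conversion math and Tiles lookup unconnected.
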(fn WorldLocationtoTile
  (params (WorldLocation :type Vector))
  (Development|PrintString 0 (Utilities|String|ToString(Vector) WorldLocation) true true "(R=0.000000,G=0.660000,B=1.000000,A=1.000000)" 0.0)
  (return 0))

(fn CreateTiles
  (bind _tilesize (Variables|Default|GetTileSize))
  (for _index (range 0 (Variables|Default|GetNumOfRows))
    (for _index_2 (range 0 (Variables|Default|GetNumOfColumns))
      (bind _returnvalue (Game|ConstructObjectfromClass "/Game/MerchantTD/Blueprint/UObjects/UTile.UTile_C" self _index_2 _index (Math|Vector|MakeVector (- (* _index_2 _tilesize) (/ (* (Variables|Default|GetNumOfColumns) (Variables|Default|GetTileSize)) 2.0)) (- (* _index _tilesize) (/ (* (Variables|Default|GetNumOfRows) (Variables|Default|GetTileSize)) 2.0)) 0.0)))
      (Utilities|Array|Add (Variables|Default|GetTiles) _returnvalue))))