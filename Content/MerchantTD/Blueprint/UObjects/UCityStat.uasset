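; UCityStat is a levelling city stat object that tracks a value against a maximum.
; Add calls LevelUp when the amount would reach Max, which increments the level, grows Max, resets Value and fires OnFull.
; It then adds the whole amount, clamped to Max, and updates Percentage, effectively a Value/Max ratio, printing it for debug.
; Subtract is an empty stub.
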(fn Add
  (params (Amount :type Float%20%28single-precision%29))
  (bind _max (Variables|Default|GetMax))
  (if (>= (/ (+ Amount (Variables|Default|GetValue)) _max) 1.0)
    (CallFunction|LevelUp))
  (Variables|Default|SetValue (Math|Float|Clamp(Float) (+ Amount (Variables|Default|GetValue)) 0.0 _max))
  (CallFunction|UpdatePercentage))

(fn Subtract
  (params (Amount :type Float%20%28single-precision%29)))

(fn LevelUp
  (Math|Integer|IncrementInt (Variables|Default|GetLv)
    (:%20%20
      (Variables|Default|SetMax (* (Variables|Default|GetMax) 1.5))
      (Variables|Default|SetValue 0.0)
      (Default|CallOnFull))))

(fn UpdatePercentage
  (bind _output_get (Variables|Default|SetPercentage (* (/ (Variables|Default|GetValue) (* (Variables|Default|GetMax) 1e+02)) 1e+02)))
  (Development|PrintString 0 (Utilities|String|ToString(Float) _output_get)))