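; UCity is the object holding a city's funds and Food stat, with functions to add money or subtract it when affordable.
; Initialize creates the UCityStat and binds to its full event; the StatFull event in the graph is empty.
; RegisterMarket binds to a market's transaction event, and ParseTransaction adds a fixed amount of Food.
; The per-resource loop and ID match in ParseTransaction are disconnected, so transaction contents are ignored.
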(event Custom|StatFull)

(event Custom|OnMarketTransaction
  (params (Transaction :type ST%20Transaction%20Structure))
  (CallFunction|ParseTransaction))

(fn Initialize
  (bind _returnvalue (Game|ConstructObjectfromClass "/Game/MerchantTD/Blueprint/UObjects/UCityStat.UCityStat_C" self "Food"))
  (bind _output_get (Variables|Default|SetFoodStat _returnvalue))
  (EventDispatchers|BindEventtoOnFull _output_get (EventDispatchers|CreateEvent :!event Custom|StatFull)))

(fn RegisterMarket
  (params (Market :type BP%20Market%20Object%20Reference))
  (Utilities|IsValid Market
    (:Is%20Valid
      (EventDispatchers|BindEventtoOnTransaction Market (EventDispatchers|CreateEvent :!event Custom|OnMarketTransaction)))))

(fn ParseTransaction
  (params (Transaction :type ST%20Transaction%20Structure))
  (Default|Add (Variables|Default|GetFoodStat) 5.0))

(fn AddFunds
  (params (Amount :type Float%20%28single-precision%29))
  (Variables|Default|SetMoney (+ Amount (Variables|Default|GetMoney))))

(fn SubtractFunds
  (params (Amount :type Float%20%28single-precision%29))
  (if (>= (Variables|Default|GetMoney) Amount)
    (Variables|Default|SetMoney (- (Variables|Default|GetMoney) Amount))
    (return true)
    (else
      (return false))))